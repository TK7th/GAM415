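; Blueprint that animates a lens distortion UV displacement map by drawing it to render target RT_00.
; Tick, throttled by a short Delay, clears the target and redraws it from a FooCameraModel built with K1 and K2.
; Each pass then nudges K1 by Inc through Inward or Outward, with a delayed Switch flag reversing direction roughly every second, so the distortion oscillates.
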(event `Inward`
  ;[1 1 1] Increase (w) or Decrase (s) the UV Displacement
  (set `self.K1` (+ (`self.K1`) (`self.inc`))))

(event `Outward`
  ;[1 1 1] Increase (w) or Decrase (s) the UV Displacement
  (set `self.K1` (+ (`self.K1`) (* (`self.inc`) -1.0))))

(event `self.ReceiveTick`
  (params (DeltaSeconds :type "Float (single-precision)"))
  ;[1 1 1] Make sure to only draw the most current K1 & K2 input values
  (`KismetSystemLibrary.Delay` 0.1)
  (`KismetRenderingLibrary.ClearRenderTarget2D` "/Game/Blueprints/RT_00.RT_00")
  (`LensDistortionBlueprintLibrary.DrawUVDisplacementToRenderTarget` (make `FooCameraModel` (`self.K1`) (`self.K2`)) 1.0 1.0 1.0 "/Game/Blueprints/RT_00.RT_00")
  (if (`self.Switch`)
    (`self.Inward`)
    (`KismetSystemLibrary.Delay` 1.0)
    (set `self.Switch` false)
    (else
      (`self.Outward`)
      (`KismetSystemLibrary.Delay` 1.0)
      (set `self.Switch` true))))

(fn `UserConstructionScript`)