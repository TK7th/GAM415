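; Game mode for the start menu that continuously randomizes Red, Green and Blue values, with no consumer of them in this graph.
; Tick runs through a 0.1 second Delay, which throttles updates to roughly ten per second.
; After each delay, three custom events each set one channel to a random float between zero and one.
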(event `self.ReceiveTick`
  (params (DeltaSeconds :type "Float (single-precision)"))
  (`KismetSystemLibrary.Delay` 0.1)
  (`self.ChangeRed`)
  (`self.ChangeGreen`)
  (`self.ChangeBlue`))

(event `ChangeRed`
  (set `self.Red` (`KismetMathLibrary.RandomFloatInRange` 0.0 1.0)))

(event `ChangeGreen`
  (set `self.Green` (`KismetMathLibrary.RandomFloatInRange` 0.0 1.0)))

(event `ChangeBlue`
  (set `self.Blue` (`KismetMathLibrary.RandomFloatInRange` 0.0 1.0)))

(fn `UserConstructionScript`)