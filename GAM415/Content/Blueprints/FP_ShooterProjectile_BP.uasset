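; Paintball projectile for a first-person shooter that leaves a randomized paint splat where it hits.
; On Hit it plays a splat sound and spawns a temporary decal at the impact point, oriented to the surface normal with a random size.
; A dynamic material instance on the decal randomizes the splat frame and color, then the projectile destroys itself.
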(event `self.ReceiveHit`
  (params (MyComp :type "PrimitiveComponent Object Reference") (Other :type "Actor Object Reference") (OtherComp :type "PrimitiveComponent Object Reference") (bSelfMoved :type Boolean) (HitLocation :type "Vector Structure") (HitNormal :type "Vector Structure") (NormalImpulse :type "Vector Structure") (Hit :type "HitResult Structure (by ref)"))
  ;[0.2512 0.5701 0] Comment
  (`GameplayStatics.PlaySoundAtLocation` "/Game/Audio/Splat_-_Audio_Cue.Splat_-_Audio_Cue" HitLocation)
  (bind _returnvalue (`GameplayStatics.SpawnDecalAtLocation` "/Game/Materials/PaintballSplat_M.PaintballSplat_M" (`KismetMathLibrary.Conv_DoubleToVector` (`KismetMathLibrary.RandomFloatInRange` 25.0 60.0)) HitLocation (`KismetMathLibrary.Conv_VectorToRotator` HitNormal) 20.0))
  (bind _returnvalue_2 (`DecalComponent.CreateDynamicMaterialInstance` _returnvalue))
  (`MaterialInstanceDynamic.SetScalarParameterValue` _returnvalue_2 "Frame" (`KismetMathLibrary.Conv_IntToDouble` (`KismetMathLibrary.RandomIntegerInRange` 0 3)))
  (`MaterialInstanceDynamic.SetVectorParameterValue` _returnvalue_2 "Color" (`KismetMathLibrary.MakeColor` (`KismetMathLibrary.RandomFloatInRange` 0.0 1.0) (`KismetMathLibrary.RandomFloatInRange` 0.0 1.0) (`KismetMathLibrary.RandomFloatInRange` 0.0 1.0)))
  (`self.K2_DestroyActor`))

(fn `UserConstructionScript`)