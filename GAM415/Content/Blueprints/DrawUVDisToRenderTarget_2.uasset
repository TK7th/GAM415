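; Blueprint that animates a lens-distortion UV displacement map drawn into render target RT_01.
; Each Tick clears the target and redraws it with DrawUVDisplacementToRenderTarget, using a camera model built from the current K1 and K2.
; Tick also steps K1 up or down by Inc through Inward and Outward, while Delay nodes flip Switch every few seconds so the distortion oscillates.
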(event `Inward`
  ;[0.1546 0.6667 0] Increase or Decrase the UV Displacement
  (set `self.K1` (+ (`self.K1`) (`self.inc`))))

(event `Outward`
  ;[0.1546 0.6667 0] Increase or Decrase the UV Displacement
  (set `self.K1` (+ (`self.K1`) (* (`self.inc`) -1.0))))

(event `self.ReceiveTick`
  (params (DeltaSeconds :type "Float (single-precision)"))
  ;[0 0.8116 0.009662] Make sure to only draw the most current K1 & K2 input values
  (`KismetRenderingLibrary.ClearRenderTarget2D` "/Game/Shaders/RT_01.RT_01")
  (`LensDistortionBlueprintLibrary.DrawUVDisplacementToRenderTarget` (make `FooCameraModel` (`self.K1`) (`self.K2`) 0.0 0.0 0.0 (0.5 0.5)) 1.0 1.0 1.0 "/Game/Shaders/RT_01.RT_01")
  (if (`self.Switch`)
    (`self.Inward`)
    (`KismetSystemLibrary.Delay` 7.0)
    (set `self.Switch` false)
    (else
      (`self.Outward`)
      (`KismetSystemLibrary.Delay` 7.0)
      (set `self.Switch` true))))

(fn `UserConstructionScript`)