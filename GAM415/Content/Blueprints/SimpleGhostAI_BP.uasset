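; SimpleGhostAI_BP is a ghost enemy that paintballs can kill for points and that hurts the player on contact.
; Each projectile hit lowers its health and launches it randomly, then recolors it through a new dynamic material instance.
; When health equals exactly zero, it destroys itself and adds points to the game mode.
; Player overlap damage sits behind a DoOnce with no reset, so it applies only once per ghost.
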(event `self.CapsuleComponent.OnComponentHit`
  (params (HitComponent :type "PrimitiveComponent Object Reference") (OtherActor :type "Actor Object Reference") (OtherComp :type "PrimitiveComponent Object Reference") (NormalImpulse :type "Vector Structure") (Hit :type "HitResult Structure (by ref)"))
  ;[0.7923 0 0.02933] When paintball makes contact with ghost, deduct 20hp and knock back ghost
  (cast `/Game/Blueprints/FP_ShooterProjectile_BP` OtherActor)
  (set `self.Health` (- (`self.Health`) 50))
  (`self.LaunchCharacter` (`KismetMathLibrary.MakeVector` (`KismetMathLibrary.RandomFloatInRange` 0.0 500.0) (`KismetMathLibrary.RandomFloatInRange` 0.0 500.0) (`KismetMathLibrary.RandomFloatInRange` 0.0 500.0)))
  (if (== (`self.Health`) 0)
    (`self.K2_DestroyActor`)
    (bind _asgam415game_mode_base_bp (cast `/Game/Blueprints/GAM415GameModeBase_BP` (`GameplayStatics.GetGameMode`)))
    (set `/Game/Blueprints/GAM415GameModeBase_BP.Points` (+ (`/Game/Blueprints/GAM415GameModeBase_BP.Points` _asgam415game_mode_base_bp) (`self.AddedPoints`)) _asgam415game_mode_base_bp)
    (else
      (bind _returnvalue (`PrimitiveComponent.CreateDynamicMaterialInstance` (`self.StaticMesh`) 0 "/Game/Materials/Ghost_M.Ghost_M"))
      (`MaterialInstanceDynamic.SetVectorParameterValue` _returnvalue "Color" (`KismetMathLibrary.MakeColor` (`KismetMathLibrary.RandomFloatInRange` 0.0 1.0) (`KismetMathLibrary.RandomFloatInRange` 0.0 1.0) (`KismetMathLibrary.RandomFloatInRange` 0.0 1.0))))))

(event `self.CapsuleComponent.OnComponentBeginOverlap`
  (params (OverlappedComponent :type "PrimitiveComponent Object Reference") (OtherActor :type "Actor Object Reference") (OtherComp :type "PrimitiveComponent Object Reference") (OtherBodyIndex :type Integer) (bFromSweep :type Boolean) (SweepResult :type "HitResult Structure (by ref)"))
  ;[0 0.686 0.1353] Deduct 20HP from player health whenever contact is made
  (bind _asfp_shooter_character_bp (cast `/Game/Blueprints/FP_ShooterCharacter_BP` OtherActor))
  (`/Engine/EditorBlueprintResources/StandardMacros.DoOnce` false
    (:`Completed`
      (set `/Game/Blueprints/FP_ShooterCharacter_BP.Health` (- (`/Game/Blueprints/FP_ShooterCharacter_BP.Health` _asfp_shooter_character_bp) 20.0) _asfp_shooter_character_bp))))

(fn `UserConstructionScript`)