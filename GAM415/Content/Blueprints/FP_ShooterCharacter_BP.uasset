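; First-person shooter player character with a stamina-limited sprint, a color-cycling gun and feedback on ghost contact.
; Tick, throttled by a half-second Delay, randomizes the gun's BodyColor via a dynamic material instance and drains or regenerates Stamina.
; Left Shift raises walk speed until stamina empties, and regeneration waits a few seconds after release.
; Overlapping a SimpleGhostAI_BP plays a hurt sound and briefly raises DamageContact for a red screen flash.
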(event `self.ReceiveTick`
  (params (DeltaSeconds :type "Float (single-precision)"))
  ;[0.3672 0 0.4595] Changes colors of first person shooter's gun
  (`KismetSystemLibrary.Delay` 0.5)
  (bind _returnvalue (`PrimitiveComponent.CreateDynamicMaterialInstance` (`self.FP_Gun`) 0 "/Game/FirstPerson/FPWeapon/Materials/M_FPGun.M_FPGun"))
  (`MaterialInstanceDynamic.SetVectorParameterValue` _returnvalue "BodyColor" (`KismetMathLibrary.MakeColor` (`KismetMathLibrary.RandomFloatInRange` 0.0 1.0) (`KismetMathLibrary.RandomFloatInRange` 0.0 1.0) (`KismetMathLibrary.RandomFloatInRange` 0.0 1.0)))
  (if (`self.isPressed`)
    (`self.Sprinting`)
    (elif (== (`self.isPressed`) (`self.BoostDelay`))
      (`self.NotSprinting`))))

(event `self.CapsuleComponent.OnComponentBeginOverlap`
  (params (OverlappedComponent :type "PrimitiveComponent Object Reference") (OtherActor :type "Actor Object Reference") (OtherComp :type "PrimitiveComponent Object Reference") (OtherBodyIndex :type Integer) (bFromSweep :type Boolean) (SweepResult :type "HitResult Structure (by ref)"))
  ;[0 0.09662 0.7247] Red flashes to the screen whenever player makes contact with ghost
  (cast `/Game/Blueprints/SimpleGhostAI_BP` OtherActor)
  (`GameplayStatics.PlaySoundAtLocation` "/Game/Audio/OUCH_Sound_Effect-YVf9wo8WZzM.OUCH_Sound_Effect-YVf9wo8WZzM")
  (set `self.DamageContact` 0.5)
  (`KismetSystemLibrary.Delay` 0.2)
  (set `self.DamageContact` 0.0))

(event `Sprinting`
  (bind _stamina (`self.Stamina`))
  ;[0.3575 0 0.4693] Reduces stamina while shift is being pressed
  (if (<= (`self.Stamina`) 100.0)
    (set `self.Stamina` (- _stamina 5.0))
    (if (<= _stamina 0.0)
      (set `self.Stamina` 0.0)
      (set `CharacterMovementComponent.MaxWalkSpeed` 400.0 (`self.CharacterMovement`)))))

(event `Key|LeftShift`
  (params (Key :type "Key Structure"))
  (bind _charactermovement (`self.CharacterMovement`))
  ;[0.7633 0 0.05866] Determine speed of player movement when sprint button is pressed or not
  (:`Pressed`
    (set `CharacterMovementComponent.MaxWalkSpeed` 850.0 _charactermovement)
    (set `self.isPressed` true)
    (set `self.BoostDelay` true))
  (:`Released`
    (set `CharacterMovementComponent.MaxWalkSpeed` 400.0 _charactermovement)
    (set `self.isPressed` false)
    (`KismetSystemLibrary.Delay` 3.0)
    (if (== (`self.isPressed`) false)
      (set `self.BoostDelay` false))))

(event `NotSprinting`
  (bind _stamina (`self.Stamina`))
  ;[0.04831 0.773 0] Regenerate stamina while shift isn't being pressed
  (if (>= (`self.Stamina`) 0.0)
    (set `self.Stamina` (+ _stamina 10.0))
    (if (>= _stamina 100.0)
      (set `self.Stamina` 100.0))))

(fn `UserConstructionScript`)